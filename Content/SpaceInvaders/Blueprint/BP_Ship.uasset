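; Player-flown physics ship for the SpaceInvaders game that fires BP_Rocket from an arrow component on left click.
; Input axes apply pitch, yaw and roll torque, while Thrust eases toward a throttle target that SuperSonic greatly raises.
; Tick overwrites physics velocity with forward plus upward velocity, though the upward term's zeroed Lerp leaves it inert.
; BeginPlay adds a health bar widget; damage lowers Health and only prints it or "Dead".
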(event Game|Damage|EventAnyDamage
  (params (Damage :type Float%20%28single-precision%29) (DamageType :type Damage%20Type%20Object%20Reference) (InstigatedBy :type Controller%20Object%20Reference) (DamageCauser :type Actor%20Object%20Reference))
  ;[1 1 1] Health Settings
  (Variables|Default|Sethealth (- (Variables|Default|Gethealth) Damage))
  (if (<= (Variables|Default|Gethealth) 0.0)
    (Development|PrintString "Dead")
    (else
      (Development|PrintString (Utilities|String|ToString(Float) (Variables|Default|Gethealth))))))

(event EventTick
  (params (DeltaSeconds :type Float%20%28single-precision%29))
  (Utilities|FlowControl|Sequence
    (:then_0
      (if (< (Math|Vector|VectorLength (Variables|Default|GetForwardVelocity)) (Variables|Default|GetGravityThreshold))
        (Variables|Default|SetUpwardsVelocity (* (Math|Float|Lerp 0.0 0.0 (- (Math|Vector|VectorLength (Variables|Default|GetForwardVelocity)) (Variables|Default|GetGravityThreshold))) (Math|Vector|UnrotateVector (Math|Vector|GetUpVector (Variables|Default|GetShip)) (Transformation|GetWorldRotation (Variables|Default|GetShip)))))
        (else
          (Variables|Default|SetUpwardsVelocity (Math|Interpolation|VInterpTo (Variables|Default|GetUpwardsVelocity) "0, 0, 0" (Utilities|Time|GetWorldDeltaSeconds) 2e+01)))))
    (:then_1
      (Physics|SetPhysicsLinearVelocity (Variables|Default|GetShip) (+ (Variables|Default|GetForwardVelocity) (Variables|Default|GetUpwardsVelocity)) false "None"))))

(event EventBeginPlay
  ;[1 1 1] Initial Thrust & Healthbar
  (bind _returnvalue (UserInterface|CreateWidget "/Game/SpaceInvaders/Blueprint/WP_HealthBar.WP_HealthBar_C" (Game|GetPlayerController 0)))
  (UserInterface|Viewport|AddtoViewport _returnvalue 0)
  (Variables|Default|SetThrust (/ (Variables|Default|GetMaxThrust) 0.0)))

(event Input|ActionEvents|InputActionSuperSonic
  (params (Key :type Key%20Structure :default "None"))
  ;[1 1 1] SuperSonic Speed
  (:Pressed
    (bind _output_get (Variables|Default|SetSuperSpeed true)))
  (:Released
    (Variables|Default|SetSuperSpeed false)))

(event Input|AxisEvents|InputAxisThrust
  (params (AxisValue :type Float%20%28single-precision%29))
  ;[1 1 1] Initial Movement
  (Utilities|FlowControl|Sequence
    (:then_0
      (if (stale Input|ActionEvents|InputActionSuperSonic _output_get)
        ;[1 1 1] SuperSonic Speed
        (if (not (Math|Float|NearlyEqual(Float) AxisValue 0.0 0.1))
          (Variables|Default|SetThrust (Math|Interpolation|FInterpTo (Variables|Default|GetThrust) (Math|Float|Lerp 0.0 (Variables|Default|GetMaxThrust) (/ (+ AxisValue 1.0) 0.1)) (Utilities|Time|GetWorldDeltaSeconds) 5.0)))
        (elif (not (Math|Float|NearlyEqual(Float) AxisValue 0.0 0.1))
          (Variables|Default|SetThrust (Math|Interpolation|FInterpTo (Variables|Default|GetThrust) (Math|Float|Lerp 0.0 (Variables|Default|GetMaxThrust) (/ (+ AxisValue 1.0) 2.0)) (Utilities|Time|GetWorldDeltaSeconds) 5.0)))))
    (:then_1
      (Variables|Default|SetForwardVelocity (* (Math|Vector|GetForwardVector (Variables|Default|GetShip)) (Variables|Default|GetThrust))))))

(event Input|AxisEvents|InputAxisMoveUp
  (params (AxisValue :type Float%20%28single-precision%29))
  (Class|PrimitiveComponent|AddTorqueinDegrees (Variables|Default|GetShip) (* (Math|Vector|GetRightVector (Variables|Default|GetShip)) (* AxisValue (Variables|Default|GetForwardTorquePower))) "None" true))

(event Input|AxisEvents|InputAxisMoveRight
  (params (AxisValue :type Float%20%28single-precision%29))
  (Class|PrimitiveComponent|AddTorqueinDegrees (Variables|Default|GetShip) (* (Math|Vector|GetUpVector (Variables|Default|GetShip)) (* AxisValue (Variables|Default|GetForwardTorquePower))) "None" true))

(event Input|AxisEvents|InputAxisRoll
  (params (AxisValue :type Float%20%28single-precision%29))
  (Class|PrimitiveComponent|AddTorqueinDegrees (Variables|Default|GetShip) (* (Math|Vector|GetForwardVector (Variables|Default|GetShip)) (* AxisValue (Variables|Default|GetForwardTorquePower))) "None" true))

(event Input|MouseEvents|LeftMouseButton
  (params (Key :type Key%20Structure :default "None"))
  (:Pressed
    (Game|SpawnActorfromClass "/Game/SpaceInvaders/SpaceShip/Projectile/BP_Rocket.BP_Rocket_C" (Transformation|GetWorldTransform (Variables|Default|GetArrow1)) "AlwaysSpawn" "MultiplyWithRoot" self 1e+03 0.0 0)))

(fn ConstructionScript)